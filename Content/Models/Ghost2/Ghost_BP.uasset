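; Ghost enemy AI that wanders to random nearby points, chases the first-person player on sight and triggers a game-over scare on catching them.
; PawnSensing starts the chase and its audio, while a retriggerable delay and Tick checks detect lost sight, fade the audio and resume wandering.
; On a catch, a self-calling delayed loop turns the player toward the ghost as it plays a montage, fades the camera and shows the Ghosted widget.
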(event `self.ReceiveBeginPlay`
  (bind _returnvalue (`AddComponent|NODE_AddAudioComponent-0`))
  (`AudioComponent.Stop` _returnvalue)
  (set `self.Audio` _returnvalue))

(event `self.PawnSensing.OnSeePawn`
  (params (Pawn :type "Pawn Object Reference"))
  (bind _asbp_first_person_character (cast `/Game/FirstPerson/Blueprints/BP_FirstPersonCharacter` Pawn))
  (if (not (`self.Caught?`))
    (`|ExecutionSequence`
      (:`then_0`
        (set `self.Can see enemy?` true)
        (set `self.IsChasing?` true)
        (`|AIMoveTo` self (0.0 0.0 0.0) _asbp_first_person_character
          (:`then`
            (`/Engine/EditorBlueprintResources/StandardMacros.DoOnce` false :!label _label
              (:`Completed`
                (`AudioComponent.Play` (`self.Audio`) 0.0))))
          (:`OnSuccess`
            (`self.Catch Player`))))
      (:`then_1`
        (`KismetSystemLibrary.RetriggerableDelay` 0.6)
        (set `self.Can see enemy?` false)))))

(event `self.ReceiveTick`
  (params (DeltaSeconds :type "Float (single-precision)"))
  (`|ExecutionSequence`
    (:`then_0`
      (if (not (`self.Can see enemy?`))
        (`KismetSystemLibrary.Delay` 0.4)
        (if (not (`self.Can see enemy?`))
          (`AudioComponent.FadeOut` (`self.Audio`) 0.5 0.0 "Linear")
          (set `self.IsChasing?` false)
          (goto _label :!via `Reset`))))
    (:`then_1`
      (if (not (`self.IsChasing?`))
        (`KismetSystemLibrary.Delay` (`KismetMathLibrary.RandomFloatInRange` 2.0 5.0))
        (`|AIMoveTo` self (`NavigationSystemV1.K2_GetRandomReachablePointInRadius` (`self.K2_GetActorLocation`) 1500.0 null null) null)))))

(event `Rotation Loop`
  (bind _returnvalue (`GameplayStatics.GetPlayerController` 0))
  (if (`self.Should Loop?`) :!label _label_2
    (`KismetSystemLibrary.Delay` 0.001)
    (bind _returnvalue_2 (`KismetMathLibrary.FindLookAtRotation` (`self.K2_GetActorLocation` (stale `Catch Player` _asbp_first_person_character)) (`self.K2_GetActorLocation`)))
    (`self.K2_SetActorRotation` (stale `Catch Player` _asbp_first_person_character) (`KismetMathLibrary.RInterpTo` (`self.K2_GetActorRotation` (stale `Catch Player` _asbp_first_person_character)) _returnvalue_2 (`GameplayStatics.GetWorldDeltaSeconds`) 5.0) false)
    (`Controller.SetControlRotation` _returnvalue (`KismetMathLibrary.RInterpTo` (`Controller.GetControlRotation` _returnvalue) _returnvalue_2 (`GameplayStatics.GetWorldDeltaSeconds`) 5.0))
    (`self.Rotation Loop`)
    (`/Engine/EditorBlueprintResources/StandardMacros.DoOnce` false :!label _label_3
      (:`Completed`
        (`|ExecutionSequence`
          (:`then_0`
            (`|PlayMontage` null "/Game/Animation/GhostAnimMontage.GhostAnimMontage"
              (:`then`
                (`KismetSystemLibrary.Delay` 0.2)
                (`PlayerCameraManager.StartCameraFade` :`self` (`GameplayStatics.GetPlayerCameraManager` 0) :`Duration` 2.0 :`bShouldFadeAudio` true :`bHoldWhenFinished` true)
                (bind _returnvalue_3 (`|CreateWidget` "/Game/UI/WBP_Ghosted.WBP_Ghosted_C"))
                (`UserWidget.AddToViewport` _returnvalue_3 0)
                (`WidgetBlueprintLibrary.SetInputMode_UIOnlyEx` null null)
                (`CharacterMovementComponent.DisableMovement` (`Character.CharacterMovement` (`GameplayStatics.GetPlayerCharacter` 0)))
                (set `self.Caught?` false))))
          (:`then_1`
            (`KismetSystemLibrary.Delay` 0.5)
            (set `self.Should Loop?` false)
            (goto _label_3 :!via `Reset`)))))))

(event `Catch Player`
  (set `self.Caught?` true)
  (set `self.Should Loop?` true)
  (bind _asbp_first_person_character (cast `/Game/FirstPerson/Blueprints/BP_FirstPersonCharacter` (`GameplayStatics.GetPlayerCharacter` 0)))
  (goto _label_2))

(fn `UserConstructionScript`)